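; BP_QuestDispenser is a talkable Blueprint that shows dialogue lines from its Kwestie array in an on-screen window.
; Each Talk event increments Index and, while it is within the array, writes that line into the TalkText of a WB_DialogueWindow.
; The widget is created lazily for player 0 and reused.
; Once the lines run out, Talk leaves the window as it is, and no quest logic is present.
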(event EventTalk
  (Math|Integer|IncrementInt (Variables|Default|GetIndex)
    (:%20%20
      (if (< (Variables|Default|GetIndex) (Utilities|Array|Length (Variables|Default|GetKwestie)))
        (Variables|Default|GetUI
          (:then
            _)
          (:else
            (bind _returnvalue (UserInterface|CreateWidget "/Game/WB_DialogueWindow.WB_DialogueWindow_C" (Game|GetPlayerController 0)))
            (bind _output_get (Variables|Default|SetUI _returnvalue))
            (UserInterface|Viewport|AddtoViewport _output_get 0)))
        (Rendering|Components|TextRender|SetText (Variables|/Game/WB_DialogueWindow.WB_DialogueWindow_C|GetTalkText (Variables|Default|GetUI)) (Utilities|Text|ToText(String) (Utilities|Array|Get(acopy) (Variables|Default|GetKwestie) (Variables|Default|GetIndex))))))))

(fn ConstructionScript)